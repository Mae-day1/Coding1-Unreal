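; BP_SpawnManager runs wave-based enemy spawning, starting the first wave shortly after BeginPlay.
; SpawnEnemies loops over every BP_SpawnPoint in the level and usually, by weighted chance, spawns a BP_Enemy at its transform.
; Dying enemies call NewWaveCheck, which counts remaining BP_Enemy actors, allowing for the dying one, and starts a new wave after a delay if none remain.
; Print strings trace each step for debugging.
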(event Custom|Spawn%20Enemies
  (bind _outactors (Actor|GetAllActorsOfClass "/Game/Blueprints/BP_SpawnPoint.BP_SpawnPoint_C")) ; get an array of all spawn points in the level
  (for _array_element _outactors ; for each element in the array, do things
    (Development|PrintString (Utilities|GetDisplayName _array_element) true true "(R=0.199773,G=0.633680,B=0.385962,A=1.000000)" 1e+01) ; print the name
    (if (Math|Random|RandomBoolwithWeight 0.8) ; chance to not spawn an enemy
      (Game|SpawnActorfromClass "/Game/Blueprints/BP_Enemy.BP_Enemy_C" (Transformation|GetWorldTransform (Variables|/Game/Blueprints/BP_SpawnPoint.BP_SpawnPoint_C|GetDefaultSceneRoot _array_element)) "Undefined" "MultiplyWithRoot" 0 0) ; spawn actor from class bp_enemy at the spawnpoint's location
    ))
  (Development|PrintString "Finished with the For Each Loop for spawn enemies."))

(event Custom|NewWaveCheck
  (Development|PrintString "Was that the last enemy?")
  (bind _outactors (Actor|GetAllActorsOfClass "/Game/Blueprints/BP_Enemy.BP_Enemy_C")) ; get an array of all BP_enemy's in the level
  (Development|PrintString (Utilities|String|Append "There are " (Utilities|String|ToString(Integer) (Utilities|Array|Length _outactors)) " enemies in the level."))
  (if (> (Utilities|Array|Length _outactors) 1) ; are there more than zero enemies?
    (Development|PrintString "You were not the last one.") ; it's not time for new enemies yet.
    (else
      (Development|PrintString "New Wave incoming!" true true "(R=1.000000,G=0.055556,B=0.091755,A=1.000000)")
      (Utilities|FlowControl|Delay 3.0) ; wait 3 seconds
      (CallFunction|SpawnEnemies) ; spawn enemies again
    )))

(event EventBeginPlay
  (Development|PrintString "Spawn Manager exists.") ; tell the player that we exist
  (Utilities|FlowControl|Delay 1.0) ; wait for some time
  (CallFunction|SpawnEnemies) ; call the spawn enemies event
)

(fn ConstructionScript)